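; Stage camera actor that keeps the player and a second fighter (BP_Fighter2Spawn) framed by following their midpoint.
; BeginPlay records their starting separation and snaps the camera behind the midpoint at a set height, aimed at it.
; Each tick scales the base camera distance by the clamped separation ratio and lerps location back along the forward vector from the current midpoint, leaving rotation unchanged.
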(event EventBeginPlay
  (bind _returnvalue (Actor|GetActorOfClass "/Game/ThirdPerson/Blueprints/BP_Fighter2Spawn.BP_Fighter2Spawn_C"))
  (bind _output_get (Variables|Default|SetFighter2 _returnvalue))
  (bind _output_get_2 (Variables|Default|SetPlayer (Game|GetPlayerCharacter 0)))
  (Variables|Default|SetBaseFighterDistance (Transformation|GetSquaredDistanceTo _output_get_2 _output_get))
  (bind _output_get_3 (Variables|Default|SetBaseMidPoint (* (+ (Transformation|GetActorLocation (Variables|Default|GetPlayer)) (Transformation|GetActorLocation (Variables|Default|GetFighter2))) 0.5)))
  (bind (_targetlocation _targetrotation) (CallFunction|CalculateCameraStartLocation _output_get_3))
  (Variables|Default|SetBaseCameraLocation _targetlocation)
  (Transformation|SetActorLocationAndRotation (Variables|Default|GetBaseCameraLocation) _targetrotation false true))

(event EventTick
  (params (DeltaSeconds :type Float%20%28single-precision%29))
  (CallFunction|UpdateCameraLocation DeltaSeconds))

(fn ConstructionScript)

(fn CalculateCameraStartLocation
  (params (MidPoint :type Vector))
  (bind _returnvalue (Transformation|GetActorForwardVector))
  (bind _basecameradistance (Variables|Default|GetBaseCameraDistance))
  (bind _camerabasezoffset (Variables|Default|GetCameraBaseZOffset))
  (bind _returnvalue_2 (* _returnvalue _basecameradistance))
  (bind _returnvalue_3 (* _returnvalue_2 -1.0))
  (bind _returnvalue_4 (+ MidPoint _returnvalue_3))
  (bind (_x _y) (Math|Vector|BreakVector _returnvalue_4))
  (bind _returnvalue_5 (Math|Vector|MakeVector _x _y _camerabasezoffset))
  (return _returnvalue_5 (Math|Rotator|MakeRotfromX (Math|Vector|Normalize (- MidPoint _returnvalue_5)))))

(fn UpdateCameraLocation
  (params (DeltaSeconds :type Float%20%28double-precision%29))
  (Utilities|FlowControl|Sequence
    (:then_0
      (LocalVariables|SetCurrentMidPoint (* (+ (Transformation|GetActorLocation (Variables|Default|GetFighter2)) (Transformation|GetActorLocation (Variables|Default|GetPlayer))) 0.5)))
    (:then_1
      (bind _output_get (LocalVariables|SetDesiredDistanceRatio (Math|Float|Clamp(Float) (Math|Float|Sqrt (/ (Transformation|GetSquaredDistanceTo (Variables|Default|GetPlayer) (Variables|Default|GetFighter2)) (Variables|Default|GetBaseFighterDistance))) (Variables|Default|GetMinDistanceRatio) (Variables|Default|GetMaxDistanceRatio))))
      (LocalVariables|SetDesiredDistance (* _output_get (Variables|Default|GetBaseCameraDistance))))
    (:then_2
      (Transformation|SetActorLocation (Math|Vector|Lerp(Vector) (Transformation|GetActorLocation) (+ (LocalVariables|GetCurrentMidPoint) (* (* (Transformation|GetActorForwardVector) -1.0) (LocalVariables|GetDesiredDistance))) (* (Variables|Default|GetLocationTurnRate) DeltaSeconds)) false false))))